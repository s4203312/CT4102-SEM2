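; AI pawn with a four-state machine that patrols or chases the player and blows itself up on reaching them.
; Tick switches on State and calls the matching event every frame, but nothing here changes State.
; Walk loops AI MoveTo between two patrol points with short pauses.
; Chase moves to the player, then spawns explosion effects and destroys the pawn, while Search and Stop are empty.
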(event Custom|Chase
  (bind _returnvalue (Transformation|GetActorLocation))
  (AI|AIMoveTo self "0, 0, 0" (Game|GetPlayerCharacter 0) 5.0 false
    (:OnSuccess
      (Effects|SpawnEmitteratLocation "/Game/StarterContent/Particles/P_Explosion.P_Explosion" _returnvalue)
      (Audio|SpawnSoundatLocation "/Game/StarterContent/Audio/Explosion_Cue.Explosion_Cue" _returnvalue "0, 0, 0" 1.0 1.0 0.0 0 0)
      (Actor|DestroyActor))))

(event Custom|Stop)

(event Custom|Walk
  (AI|AIMoveTo self (Variables|Default|GetPatrolPoint1) 0 5.0 false
    (:OnSuccess
      (Utilities|FlowControl|Delay 1.0)
      (AI|AIMoveTo self (Variables|Default|GetPatrolPoint2) 0 5.0 false
        (:OnSuccess
          (Utilities|FlowControl|Delay 1.0)
          (CallFunction|Walk))))))

(event Custom|Search)

(event EventTick
  (params (DeltaSeconds :type Float%20%28single-precision%29))
  (switch Utilities|FlowControl|Switch|SwitchonAIStates (Variables|Default|GetState)
    (:NewEnumerator0
      (CallFunction|Walk))
    (:NewEnumerator1
      (CallFunction|Chase))
    (:NewEnumerator2
      (CallFunction|Search))
    (:NewEnumerator3
      (CallFunction|Stop))))

(fn ConstructionScript)