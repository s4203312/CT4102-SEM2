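; BP_Doors is a door Blueprint with events that open and close a door by setting actor rotation, acting only for the ThirdPersonCharacter.
; OpenDoor sets the passed door to an absolute angle on the X, Y or Z axis, chosen by string.
; CloseDoor waits briefly, then resets the rotation to zero.
; SlowlyOpenDoors ignores its Rotation input and instantly sets zero rotation, with no interpolation.
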(event Custom|CloseDoor
  (params (Player :type Actor%20Object%20Reference) (Door :type Actor%20Object%20Reference))
  (Utilities|Casting|CastToThirdPersonCharacter Player)
  (Utilities|FlowControl|Delay 1.0)
  (Transformation|SetActorRotation Door))

(event Custom|OpenDoor
  (params (Player :type Actor%20Object%20Reference) (Door :type Actor%20Object%20Reference) (Rotation :type Float%20%28single-precision%29) (Axis :type String))
  (if (Utilities|Enum|Equal(Enum) Axis "X")
    (Utilities|Casting|CastToThirdPersonCharacter Player)
    (Transformation|SetActorRotation Door (Math|Rotator|MakeRotator Rotation 0.0 0.0))
    (elif (Utilities|Enum|Equal(Enum) Axis "Y")
      (Utilities|Casting|CastToThirdPersonCharacter Player)
      (Transformation|SetActorRotation Door (Math|Rotator|MakeRotator 0.0 Rotation 0.0))
      (elif (Utilities|Enum|Equal(Enum) Axis "Z")
        (Utilities|Casting|CastToThirdPersonCharacter Player)
        (Transformation|SetActorRotation Door (Math|Rotator|MakeRotator 0.0 0.0 Rotation))))))

(event Custom|SlowlyOpenDoors
  (params (Rotation :type Float%20%28single-precision%29) (Player :type Actor%20Object%20Reference))
  (Utilities|Casting|CastToThirdPersonCharacter Player)
  (Transformation|SetActorRotation (Variables|Default|GetDoor) (Math|Rotator|MakeRotator 0.0 0.0 0.0)))