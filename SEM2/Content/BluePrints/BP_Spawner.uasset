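; BP_Spawner is an actor that produces a random item at its own transform every second.
; A looping timer started on BeginPlay fires the Spawn event, which picks a random class from the Items array and spawns it.
; It then calls Clone on that temporary instance with the spawner's transform and immediately destroys the instance, leaving any lasting copy to the item's Clone implementation.
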(event Custom|Spawn
  (bind _returnvalue (Transformation|GetActorTransform))
  (bind _items (Variables|Default|GetItems))
  (bind _returnvalue_2 (Game|SpawnActorfromClass (Utilities|Array|Get(acopy) _items (Math|Random|RandomIntegerinRange 0 (- (Utilities|Array|Length _items) 1))) _returnvalue "Undefined" 0 0))
  (Default|Clone _returnvalue_2 _returnvalue)
  (Actor|DestroyActor _returnvalue_2))

(event EventBeginPlay
  (Utilities|Time|SetTimerbyEvent (delegate Custom|Spawn) 1.0 true))

(fn ConstructionScript)